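; SteamGameInstance is a game instance Blueprint that hosts and joins multiplayer sessions through Advanced Sessions nodes.
; CreateSession creates a session and, on success, opens ThirdPersonExampleMap as a listen server.
; FindSession searches all server types and joins the first result, with no selection step.
; Successful creation and joining print the local player's nickname, looked up from their unique net ID.
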(event `Create Session`
  (`CreateSessionCallbackProxyAdvanced.CreateAdvancedSession` :`PlayerController` (`GameplayStatics.GetPlayerController` 0)
    (:`OnSuccess`
      (`GameplayStatics.OpenLevel` "ThirdPersonExampleMap" true "listen")
      (`KismetSystemLibrary.PrintString` (`KismetStringLibrary.Concat_StrStr` (`AdvancedIdentityLibrary.GetPlayerNickname` (`AdvancedSessionsLibrary.GetUniqueNetID` (`GameplayStatics.GetPlayerController` 0))) " created session.")))))

(event `Find Session`
  (bind _returnvalue (`GameplayStatics.GetPlayerController` 0))
  (bind _results (`FindSessionsCallbackProxyAdvanced.FindSessionsAdvanced` (`GameplayStatics.GetPlayerController` 0) 10 false "AllServers")
    (:`OnSuccess`
      (bind _output_get (set `self.Found Sessions` _results))
      (for (_array_element _array_index) _output_get
        (if (== _array_index 0)
          (`JoinSessionCallbackProxy.JoinSession` _returnvalue _array_element
            (:`OnSuccess`
              (`KismetSystemLibrary.PrintString` (`KismetStringLibrary.Concat_StrStr` (`AdvancedIdentityLibrary.GetPlayerNickname` (`AdvancedSessionsLibrary.GetUniqueNetID` _returnvalue)) " has joined!")))))))))