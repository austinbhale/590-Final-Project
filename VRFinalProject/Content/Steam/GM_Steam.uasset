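; Game mode for a Steam multiplayer VR test that assigns pre-placed VRPawns to players.
; BeginPlay stores the first two VRPawns found and gives the first to player controller 0 with game-only input.
; PostLogin makes each joining player possess the second stored pawn.
; Advanced Sessions create, find and join logic and Steam identity prints are disconnected, leaving the CreateSession and FindSession events empty.
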(event `self.ReceiveBeginPlay`
  (bind _returnvalue (`GameplayStatics.GetPlayerController` 0))
  (`|ExecutionSequence`
    (:`then_2`
      (bind _outactors (`GameplayStatics.GetAllActorsOfClass` "/Game/a7/VRPawn.VRPawn_C"))
      (for (_array_element _array_index) _outactors
        (if (== _array_index 0)
          (set `self.Pawn` _array_element)
          (elif (== _array_index 1)
            (set `self.Pawn1` _array_element))))
      (`Controller.Possess` _returnvalue (`self.Pawn`))
      (`WidgetBlueprintLibrary.SetInputMode_GameOnly` _returnvalue))))

(event `self.K2_PostLogin`
  (params (NewPlayer :type "PlayerController Object Reference"))
  (`Controller.Possess` NewPlayer (`self.Pawn1`))
  (`WidgetBlueprintLibrary.SetInputMode_GameOnly` NewPlayer))

(event `Create Session`)

(event `Find Session`)

(fn `UserConstructionScript`)