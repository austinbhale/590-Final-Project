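; Steam game instance Blueprint that hosts and joins multiplayer sessions through Advanced Sessions nodes.
; CreateSession opens ThirdPersonExampleMap as a listen server on success.
; FindSession searches all server types and joins using the element left after an empty loop over the results.
; A custom event possesses Pawn1 for a new player, but the VRPawn lookup that assigns it is disconnected, as are the player ID debug prints.
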(event `CustomEvent_1`
  (params (DeltaSeconds :type "Float (double-precision)")))

(event `CustomEvent_2`
  (params (NewPlayer :type "PlayerController Object Reference"))
  (`Controller.Possess` NewPlayer (`self.Pawn1`))
  (`WidgetBlueprintLibrary.SetInputMode_GameOnly` NewPlayer))

(event `Create Session`
  (`CreateSessionCallbackProxyAdvanced.CreateAdvancedSession` :`PlayerController` (`GameplayStatics.GetPlayerController` 0)
    (:`OnSuccess`
      (`GameplayStatics.OpenLevel` "ThirdPersonExampleMap" true "listen"))))

(event `Find Session`
  (bind _returnvalue (`GameplayStatics.GetPlayerController` 0))
  (bind _results (`FindSessionsCallbackProxyAdvanced.FindSessionsAdvanced` _returnvalue 10 false "AllServers")
    (:`OnSuccess`
      (bind _output_get (set `self.BlueprintSessions` _results))
      (for _array_element _output_get
        _)
      (`JoinSessionCallbackProxy.JoinSession` _returnvalue _array_element))))