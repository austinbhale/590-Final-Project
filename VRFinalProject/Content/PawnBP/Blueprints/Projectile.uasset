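; Projectile actor that damages either of two VR player pawns on impact and explodes when destroyed.
; BeginPlay caches the first two VRPawn actors in the level, and a component hit on either plays a hit sound and runs UpdateHealth.
; UpdateHealth subtracts the damage amount and refreshes that pawn's health bar, only if the bar is valid.
; Any hit destroys the projectile on authority, and Destroyed spawns a pooled explosion emitter.
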(event `Update Health`
  (params (Pawn :type "/Game/a7/VRPawn Object Reference"))
  (bind _health_bar (`/Game/a7/VRPawn.Health Bar` Pawn))
  (bind _damageamount (`self.DamageAmount`))
  (if (`KismetSystemLibrary.IsValid` _health_bar)
    (bind _curr_health (`/Game/a7/VRPawn.getCurrHealth` Pawn))
    (bind _max_health (`/Game/a7/VRPawn.getMaxHealth` Pawn))
    (bind _returnvalue (- _curr_health _damageamount))
    (`/Game/a7/VRPawn.setCurrHealth` Pawn _returnvalue)
    (`/Game/PawnBP/Blueprints/UI/HealthBar.UpdateHealth` _health_bar _returnvalue (/ (- _curr_health _damageamount) _max_health))))

(event `self.Collision.OnComponentHit`
  (params (HitComponent :type "PrimitiveComponent Object Reference") (OtherActor :type "Actor Object Reference") (OtherComp :type "PrimitiveComponent Object Reference") (NormalImpulse :type "Vector Structure") (Hit :type "HitResult Structure (by ref)"))
  (bind _vrpawn (`self.VRPawn`))
  (bind _vrpawn1 (`self.VRPawn1`))
  ;[1 1 1] Update Health on VRPawn Collision with Projectile
  (bind _aspawn (cast `Pawn` OtherActor)
    (:`then`
      (if (== _vrpawn _aspawn)
        (`GameplayStatics.PlaySound2D` "/Game/PawnBP/Blueprints/Sounds/hit.hit" 1.0 1.0 0.0 null _vrpawn)
        (`self.Update Health` _vrpawn)
        (elif (== _vrpawn1 _aspawn)
          (`GameplayStatics.PlaySound2D` "/Game/PawnBP/Blueprints/Sounds/hit.hit" 1.0 1.0 0.0 null _vrpawn1)
          (`self.Update Health` _vrpawn1))))
    (:`CastFailed`
      _))
  (`/Engine/EditorBlueprintResources/ActorMacros.Switch Has Authority`
    (:`Authority`
      (`self.K2_DestroyActor`))))

(event `self.ReceiveBeginPlay`
  (bind _outactors (`GameplayStatics.GetAllActorsOfClass` "/Game/a7/VRPawn.VRPawn_C"))
  (for (_array_element _array_index) _outactors
    (if (== _array_index 0)
      (set `self.VRPawn` _array_element)
      (elif (== _array_index 1)
        (set `self.VRPawn1` _array_element)))))

(event `self.ReceiveDestroyed`
  (bind _returnvalue_location (`KismetMathLibrary.BreakTransform` (`self.GetTransform`)))
  ;[1 1 1] Spawn Explosion Particle on Destroy
  (`GameplayStatics.SpawnEmitterAtLocation` "/Game/StarterContent/Particles/P_Explosion.P_Explosion" _returnvalue_location (struct) (1.0 1.0 1.0) true "AutoRelease"))

(fn `UserConstructionScript`)