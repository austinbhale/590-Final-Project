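; Networked weapon actor that fires projectiles while fire is held, limited by ammo count.
; StartFire and EndFire forward to server events that set IsFiring.
; Authority-only Tick runs the fire-rate timer, triggers the multicast muzzle flash, and calls SpawnProjectile.
; SpawnProjectile spawns just ahead of the spawn point and decrements ammo, or prints a pickup hint when empty.
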(event `TickAuthority`
  (params (DeltaSeconds :type "Float (double-precision)"))
  ;[1 1 1] Tick Logic for Authoritative Actor Only
  (`|ExecutionSequence`
    (:`then_0`
      ;[1 1 1] Decrement Firing Timer
      (if (> (`self.FiringTimer`) 0.0)
        (set `self.FiringTimer` (- (`self.FiringTimer`) DeltaSeconds))))
    (:`then_1`
      (if (and (`self.IsFiring`) (<= (`self.FiringTimer`) 0.0))
        ;[1 1 1] Spawn Projectile and Reset Firing Timer
        (if (> (`self.ammoCount`) 0)
          (`self.ToggleVFX` true) ; Multicast VFX toggle
        )
        (`self.SpawnProjectile` "/Game/PawnBP/Blueprints/Projectile.Projectile_C") ; Projectile initializes forward motion automatically
        (set `self.FiringTimer` (`self.FireRate`))))))

(event `self.ReceiveTick`
  (params (DeltaSeconds :type "Float (single-precision)"))
  (`/Engine/EditorBlueprintResources/ActorMacros.Switch Has Authority`
    (:`Authority`
      (`self.TickAuthority` DeltaSeconds))))

(event `ToggleVFX`
  (params (Value :type Boolean))
  ;[1 1 1] Toggle VFX - Triggers muzzle flash on all machines
  (`ActorComponent.SetActive` (`self.FlashPoint`) Value true))

(event `ServerStartFire`
  ;[1 1 1] Begin and End Fire on Server
  (set `self.IsFiring` true))

(event `StartFire`
  ;[1 1 1] Start and End Fire - Called by Local Player
  (`self.ServerStartFire`))

(event `ServerEndFire`
  ;[1 1 1] Begin and End Fire on Server
  (set `self.IsFiring` false))

(event `EndFire`
  ;[1 1 1] Start and End Fire - Called by Local Player
  (`self.ServerEndFire`))

(fn `getAmmo`
  (returns (NewParam :type Integer))
  (return (`self.ammoCount`)))

(fn `OnRep_IsFiring`
  (set `self.ShouldPlayMuzzleFlash` true))

(fn `SpawnProjectile`
  (params (`Projectile Type` :type "/Game/PawnBP/Blueprints/Projectile Class Reference"))
  (bind _ammocount (`self.ammoCount`))
  (bind (_returnvalue_location _returnvalue_rotation) (`KismetMathLibrary.BreakTransform` (`SceneComponent.K2_GetComponentToWorld` (`self.ProjectileSpawnPt`))))
  (if (> _ammocount 0)
    (`|SpawnActorFromClass` `Projectile Type` (`KismetMathLibrary.MakeTransform` (+ _returnvalue_location (* (`self.GetActorForwardVector`) 20.0)) _returnvalue_rotation) "AlwaysSpawn" "OverrideRootScale" (`self.GetOwner`) (`self.GetInstigator`))
    (set `self.ammoCount` (- _ammocount 1))
    (else
      (`KismetSystemLibrary.PrintString` "Collect ammo first! Walk over ammo to collect it"))))

(fn `UserConstructionScript`)